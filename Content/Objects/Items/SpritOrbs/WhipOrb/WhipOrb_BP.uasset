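; WhipOrb_BP is a collectible spirit orb tied to Nil's whip ability, with dialogue that teaches the spin attack and grab controls.
; On BeginPlay it caches the player and the GameInstance's speech bubble, destroying itself if the whip is already unlocked.
; Collect calls the parent implementation, then on first pickup hides the orb, plays timed tutorial lines at Nil's billboard and destroys the actor.
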(event Custom|CheckCollected
  (if (Variables|/Game/Actors/Player/Nil_BP.Nil_BP_C|GetwhipUnlocked (Variables|Default|GetNil))
    (Actor|DestroyActor)))

(event EventBeginPlay
  (bind _asnil_bp (Utilities|Casting|CastToNil_BP (Game|Player|GetPlayerPawn 0)))
  (Variables|Default|SetNil _asnil_bp)
  (CallFunction|CheckCollected)
  (bind _asnil_gi (Utilities|Casting|CastToNil_GI (Game|GetGameInstance)))
  (Variables|Default|SetSpeechBubble (Variables|/Game/System/Nil_GI.Nil_GI_C|GetSpeechBubble _asnil_gi)))

(event Collision|EventActorBeginOverlap
  (params (OtherActor :type Actor%20Object%20Reference)))

(event EventTick
  (params (DeltaSeconds :type Float%20%28single-precision%29)))

(event EventCollect
  (bind _speechbubble (Variables|Default|GetSpeechBubble))
  (bind _speechbubble_2 (Variables|Default|GetSpeechBubble))
  (|CallParentFunction)
  (if (not (Variables|Default|Getcollected))
    (Rendering|SetVisibility (Variables|Default|GetWhipOrb) false false)
    (Variables|Default|Setcollected true)
    (UserInterface|Viewport|AddtoViewport _speechbubble_2 0)
    (Default|EndConversation _speechbubble_2)
    (Default|StartConversation _speechbubble_2 (Variables|/Game/Actors/Player/Nil_BP.Nil_BP_C|GetBillboard (Variables|Default|GetNil)) 25.0)
    (Default|FeedText _speechbubble_2 "Ahhhhh! That feels much better! Now that I've recovered my tensile strength, I should be able to help you out.")
    (Utilities|FlowControl|Delay 3.0)
    (Default|FeedText _speechbubble "Use LMB to have me use my super spin attack and Q to have me grab stuff. ")
    (Utilities|FlowControl|Delay 3.0)
    (Default|FeedText _speechbubble_2 "I can only latch onto spherical objects and sideways beams though. Don't ask why. Please.")
    (Utilities|FlowControl|Delay 3.0)
    (Default|EndConversation _speechbubble)
    (Actor|DestroyActor)))

(fn ConstructionScript)