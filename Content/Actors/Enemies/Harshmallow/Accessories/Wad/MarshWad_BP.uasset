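; MarshWad_BP is the Harshmallow enemy's wad projectile, which can hit the player (Nil) or be bounced back when blocked.
; After a short launch delay, Tick turns the wad mesh to follow its velocity.
; Blocking aligns it opposite the player's shield rotation, sends it away from the blocker with upward lift, and sets ShouldKill.
; While ShouldKill is set, capsule overlaps damage Nil or spawn a splatter on ground-tagged components, destroying the wad.
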(event OnComponentBeginOverlap(WadCapsule)
  (params (OverlappedComponent :type Primitive%20Component%20Object%20Reference) (OtherActor :type Actor%20Object%20Reference) (OtherComp :type Primitive%20Component%20Object%20Reference) (OtherBodyIndex :type Integer) (bFromSweep :type Boolean) (SweepResult :type Hit%20Result%20Structure%20%28by%20ref%29))
  (bind _self self)
  (bind _returnvalue (Transformation|GetActorTransform _self))
  (bind (_location _rotation _scale) (Math|Transform|BreakTransform _returnvalue))
  (if (Variables|Default|GetshouldKill)
    (bind _asnil_bp (Utilities|Casting|CastToNil_BP OtherActor)
      (:then
        (if (== OtherComp (Variables|/Script/Engine.Character|GetCapsuleComponent _asnil_bp))
          (Default|TakeHit _asnil_bp (Variables|Default|GetProjectileAtk))
          (Actor|DestroyActor)))
      (:CastFailed
        (if (Utilities|Array|ContainsItem (Variables|/Script/Engine.ActorComponent|GetComponentTags OtherComp) "ground")
          (Game|SpawnActorfromClass "/Game/Actors/Enemies/Harshmallow/Accessories/Wad/Splatter/Splatter_BP.Splatter_BP_C" (Math|Transform|MakeTransform _location "0, 0, 0" _scale) "AdjustIfPossibleButAlwaysSpawn" 0 0)
          (Actor|DestroyActor))))))

(event Custom|Launch
  (Utilities|FlowControl|Delay 0.2)
  (Variables|Default|SetisLaunched true))

(event Custom|GetBlocked
  (params (ForceSource :type Actor%20Object%20Reference))
  (CallFunction|Bounce 6 ForceSource))

(event Custom|OrientProjectileForLaunch
  (bind _asnil_bp (Utilities|Casting|CastToNil_BP (Game|Player|GetPlayerPawn 0)))
  (Transformation|SetActorRotation (Math|Rotator|MakeRotator (.Roll (Math|Rotator|BreakRotator (Variables|/Game/Actors/Player/Anims/Nil2_AB.Nil2_AB_C|GetshieldRotation (Variables|/Game/Actors/Player/Nil_BP.Nil_BP_C|GetAnims _asnil_bp)))) (+ (.Pitch (Math|Rotator|BreakRotator (Variables|/Game/Actors/Player/Anims/Nil2_AB.Nil2_AB_C|GetshieldRotation (Variables|/Game/Actors/Player/Nil_BP.Nil_BP_C|GetAnims _asnil_bp)))) 1.8e+02) (.Yaw (Math|Rotator|BreakRotator (Variables|/Game/Actors/Player/Anims/Nil2_AB.Nil2_AB_C|GetshieldRotation (Variables|/Game/Actors/Player/Nil_BP.Nil_BP_C|GetAnims _asnil_bp)))))))

(event Custom|Bounce
  (params (Knockback :type Integer) (Attacker :type Actor%20Object%20Reference))
  ;[1 1 1] Apply Bounceback to Projectile
  (CallFunction|OrientProjectileforLaunch)
  (Variables|/Script/Engine.MovementComponent|SetVelocity (Variables|Default|GetProjectileMovement) (* (+ (- (Transformation|GetActorLocation) (Transformation|GetActorLocation Attacker)) "0, 0,30.000000") 5))
  (Variables|Default|SetshouldKill true))

(event EventBeginPlay
  (Variables|Default|SetProjectileAtk 5))

(event Collision|EventActorBeginOverlap
  (params (OtherActor :type Actor%20Object%20Reference)))

(event EventTick
  (params (DeltaSeconds :type Float%20%28single-precision%29))
  (bind _returnvalue (Transformation|GetActorLocation))
  (bind _projectilemovement (Variables|Default|GetProjectileMovement))
  (bind _velocity (Variables|/Script/Engine.MovementComponent|GetVelocity _projectilemovement))
  (bind _returnvalue_2 (+ _returnvalue _velocity))
  (bind _returnvalue_3 (Math|Rotator|FindLookatRotation _returnvalue _returnvalue_2))
  (bind (_roll _pitch _yaw) (Math|Rotator|BreakRotator _returnvalue_3))
  ;[1 1 1] Update Rotation (Tick)
  (if (Variables|Default|GetisLaunched)
    (Transformation|SetWorldRotation (Variables|Default|GetWad) (Math|Rotator|MakeRotator _roll (+ _pitch 9e+01) _yaw) false false)))

(fn ConstructionScript)