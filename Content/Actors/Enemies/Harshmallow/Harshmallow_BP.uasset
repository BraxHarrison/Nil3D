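; Harshmallow is a ranged enemy that lobs MarshWad projectiles at the player and retreats when crowded.
; When PawnSensing spots the player, it moves into throwing range, holds the spawned wad weightless briefly, then launches it on a suggested high-arc velocity.
; Tick turns it away from a nearby player and moves it toward its RunAwayBox component.
; IsFleeing blocks new attacks, and MoveStun enforces a cooldown between throws.
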(event OnSeePawn(PawnSensing)
  (params (Pawn :type Pawn%20Object%20Reference))
  (if (and (not (AI|Components|NavMovement|IsFalling (Variables|Character|GetCharacterMovement))) (not (Variables|Default|GetisFleeing)))
    (CallFunction|FacePlayer)
    (AI|AIMoveTo 0 (Transformation|GetActorLocation (Variables|Default|GetPlayer)) 0 3e+02 false
      (:OnSuccess
        (if (and (not (Variables|Default|GetmoveStun)) (not (Variables|Default|GetisFleeing)))
          (CallFunction|ThrowGobs))))))

(event Custom|ThrowGobs
  (Variables|Default|SetmoveStun true)
  (Variables|Default|SetisAttacking true)
  (Utilities|FlowControl|Delay 0.2)
  (bind _returnvalue (Game|SpawnActorfromClass "/Game/Actors/Enemies/Harshmallow/Accessories/Wad/MarshWad_BP.MarshWad_BP_C" (Math|Transform|MakeTransform (Transformation|GetWorldLocation (Variables|Default|GetBillboard))) "Undefined" 0 self))
  (Game|Components|ProjectileMovement|SetVelocityinLocalSpace (Variables|/Game/Actors/Enemies/Harshmallow/Accessories/Wad/MarshWad_BP.MarshWad_BP_C|GetProjectileMovement _returnvalue) "0, 0, 0")
  (Variables|/Script/Engine.ProjectileMovementComponent|SetProjectileGravityScale (Variables|/Game/Actors/Enemies/Harshmallow/Accessories/Wad/MarshWad_BP.MarshWad_BP_C|GetProjectileMovement _returnvalue) 0.0)
  (Utilities|FlowControl|Delay 0.2)
  (Variables|/Script/Engine.ProjectileMovementComponent|SetProjectileGravityScale (Variables|/Game/Actors/Enemies/Harshmallow/Accessories/Wad/MarshWad_BP.MarshWad_BP_C|GetProjectileMovement _returnvalue) 1.0)
  (Default|Launch _returnvalue)
  (bind _tossvelocity (Class|GameplayStatics|BlueprintSuggestProjectileVelocity (Transformation|GetActorLocation _returnvalue) (Transformation|GetActorLocation (Game|Player|GetPlayerPawn 0)) 8e+02 0.0 "DoNotTrace" 0.0 true false))
  (Variables|/Script/Engine.MovementComponent|SetVelocity (Variables|/Game/Actors/Enemies/Harshmallow/Accessories/Wad/MarshWad_BP.MarshWad_BP_C|GetProjectileMovement _returnvalue) _tossvelocity)
  (Collision|IgnoreActorwhenMoving (Variables|/Game/Actors/Enemies/Harshmallow/Accessories/Wad/MarshWad_BP.MarshWad_BP_C|GetWad _returnvalue) self true)
  (Variables|Default|SetisAttacking false)
  (Utilities|FlowControl|Delay 3.0)
  (Variables|Default|SetmoveStun false))

(event EventBeginPlay
  (Variables|Default|SetHP 10)
  (Variables|Default|SetDefense 5)
  (Variables|Default|SetKnockbackDef 1)
  (bind _asnil_bp (Utilities|Casting|CastToNil_BP (Game|Player|GetPlayerPawn 0)))
  (Variables|Default|SetPlayer _asnil_bp)
  (Development|PrintString "Cast Success"))

(event Collision|EventActorBeginOverlap
  (params (OtherActor :type Actor%20Object%20Reference)))

(event EventTick
  (params (DeltaSeconds :type Float%20%28single-precision%29))
  (bind _self self)
  (bind _player (Variables|Default|GetPlayer))
  (bind _returnvalue (Transformation|GetActorRotation _self))
  (bind (_roll _pitch) (Math|Rotator|BreakRotator _returnvalue))
  (if (< (Transformation|GetDistanceTo _player) 2.5e+02)
    (Variables|Default|SetisFleeing true)
    (Transformation|SetActorRotation (Math|Rotator|MakeRotator _roll _pitch (+ (.Yaw (Math|Rotator|BreakRotator (Math|Rotator|FindLookatRotation (Transformation|GetActorLocation _self) (Transformation|GetActorLocation _player)))) 1.8e+02)))
    (AI|AIMoveTo self (Transformation|GetWorldLocation (Variables|Default|GetrunAwayBox)) 0 5.0 false)
    (else
      (Variables|Default|SetisFleeing false))))

(fn ConstructionScript)