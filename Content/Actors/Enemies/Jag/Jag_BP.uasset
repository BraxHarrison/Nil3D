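; Jag is an enemy that chases and leaps at the player, and can curl into a physics-driven ball.
; On sighting, it moves within range and launches along a suggested projectile arc, with a cooldown between leaps.
; CurlUp enables capsule physics with a small bounce; pickup extends the ball timer and attaches it to Nil's scarf socket.
; Tick counts the timer down per frame, calling UnBall at zero to stop physics and right the capsule.
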(event OnSeePawn(PawnSensing)
  (params (Pawn :type Pawn%20Object%20Reference))
  (if (Math|Boolean|ANDBoolean (not (AI|Components|NavMovement|IsFalling (Variables|Character|GetCharacterMovement))) (not (Variables|Default|GetisFleeing)) (not (Variables|Default|GetisBalled)))
    (CallFunction|FacePlayer)
    (AI|AIMoveTo self "0, 0, 0" Pawn 4e+02 false
      (:OnSuccess
        (if (and (not (Variables|Default|GetmoveStun)) (not (Variables|Default|GetisFleeing)))
          (CallFunction|Leap))))))

(event Custom|UnBall
  (bind _capsulecomponent (Variables|Default|GetCapsuleComponent))
  (Variables|Default|SetballTimer 0.0)
  (Variables|Default|SetisBalled false)
  (Physics|SetSimulatePhysics (Variables|Default|GetCapsuleComponent) false)
  (Transformation|SetWorldRotation _capsulecomponent (Math|Rotator|MakeRotator 0.0 0.0 (.Yaw (Math|Rotator|BreakRotator (Transformation|GetWorldRotation _capsulecomponent)))) false false))

(event Custom|BounceBall
  (CallFunction|ToggleIgnorePlayer true)
  (Physics|AddImpulse (Variables|Default|GetCapsuleComponent) "0,0.000000,120.000000" "None" true)
  (Utilities|FlowControl|Delay 0.2)
  (CallFunction|ToggleIgnorePlayer false))

(event Custom|Leap
  (Variables|Default|SetmoveStun true)
  (bind _tossvelocity (Class|GameplayStatics|BlueprintSuggestProjectileVelocity (Transformation|GetActorLocation) (Transformation|GetActorLocation (stale OnSeePawn(PawnSensing) Pawn)) 7e+02 0.0 "DoNotTrace" 0.0 false false))
  (Character|LaunchCharacter (Math|Vector|MakeVector (.X (Math|Vector|BreakVector _tossvelocity)) (.Y (Math|Vector|BreakVector _tossvelocity)) (+ (.Z (Math|Vector|BreakVector _tossvelocity)) 1e+02)) true false)
  (Variables|Default|SetisLeaping true)
  (Utilities|FlowControl|Delay 3.0)
  (Variables|Default|SetmoveStun false))

(event Custom|GetPickedUp
  (Variables|Default|SetballTimer 1e+01)
  (Transformation|AttachActorToActor (Variables|Default|GetNil) "scarfControl_004" "SnapToTarget" "KeepWorld" "KeepWorld" true)
  (Development|PrintString "Get Picked Up??"))

(event Custom|CurlUp
  (Variables|Default|SetballTimer 5.0)
  (Variables|Default|SetisBalled true)
  (Physics|SetSimulatePhysics (Variables|Default|GetCapsuleComponent) true)
  (CallFunction|BounceBall))

(event EventBeginPlay
  (Variables|Default|SetName "Jag")
  (Variables|Default|SetHP 15)
  (Variables|Default|SetDefense 15)
  (Variables|Default|SetKnockbackDef 1)
  (Variables|Default|Setplayer (Game|Player|GetPlayerPawn 0))
  (CallFunction|SetNil))

(event Collision|EventActorBeginOverlap
  (params (OtherActor :type Actor%20Object%20Reference)))

(event EventTick
  (params (DeltaSeconds :type Float%20%28single-precision%29))
  (if (Math|Float|NearlyEqual(Float) (Variables|Default|GetballTimer) 0.0 1e-06)
    (CallFunction|UnBall)
    (else
      (Variables|Default|SetballTimer (- (Variables|Default|GetballTimer) 0.05)))))

(fn ConstructionScript)

(fn NewFunction00)