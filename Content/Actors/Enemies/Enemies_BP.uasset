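; Base enemy Character Blueprint handling damage, knockback and hit stun.
; Overlap with a whipping Nil's weapon-tagged component triggers knockback plus damage, except Jag enemies, which curl up instead; Bramble hits only knock back.
; Damage is divided by Defense, destroying the enemy at zero HP or granting brief invincibility, then turning it toward the player.
; Knockback launches it away from the attacker, reduced by KnockbackDef, and halts AI movement.
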(event OnComponentHit(CapsuleComponent)
  (params (HitComponent :type Primitive%20Component%20Object%20Reference) (OtherActor :type Actor%20Object%20Reference) (OtherComp :type Primitive%20Component%20Object%20Reference) (NormalImpulse :type Vector :default "0, 0, 0") (Hit :type Hit%20Result%20Structure%20%28by%20ref%29))
  (bind _asbramble_bp (Utilities|Casting|CastToBramble_BP OtherActor))
  (CallFunction|TakeKnockback 10 _asbramble_bp))

(event OnComponentBeginOverlap(CapsuleComponent)
  (params (OverlappedComponent :type Primitive%20Component%20Object%20Reference) (OtherActor :type Actor%20Object%20Reference) (OtherComp :type Primitive%20Component%20Object%20Reference) (OtherBodyIndex :type Integer) (bFromSweep :type Boolean) (SweepResult :type Hit%20Result%20Structure%20%28by%20ref%29))
  (bind _asnil_bp (Utilities|Casting|CastToNil_BP OtherActor))
  (if (Variables|/Game/Actors/Player/Nil_BP.Nil_BP_C|GetisWhipping _asnil_bp)
    (if (Components|ComponentHasTag OtherComp "weapon")
      (bind _asjag_bp (Utilities|Casting|CastToJag_BP self)
        (:then
          (CallFunction|TakeKnockback (Variables|/Game/Actors/Player/Nil_BP.Nil_BP_C|GetknockBackAtk _asnil_bp) _asnil_bp)
          (Default|CurlUp _asjag_bp))
        (:CastFailed
          (CallFunction|TakeKnockback (Variables|/Game/Actors/Player/Nil_BP.Nil_BP_C|GetknockBackAtk _asnil_bp) _asnil_bp)
          (CallFunction|LoseHealth 5))))))

(event Custom|LoseHealth
  (params (Damage :type Integer))
  ;[1 1 1] Damage Enemy
  (if (not (Variables|Default|GetisInvicible))
    (Variables|Default|SetisInvicible true)
    (Variables|Default|SethitStun true)
    (Development|PrintString "The enemy is stunned!")
    (bind _output_get (Variables|Default|SetHP (- (Variables|Default|GetHP) (/ Damage (Variables|Default|GetDefense)))))
    (if (<= _output_get 0)
      (Actor|DestroyActor)
      (else
        (Utilities|FlowControl|Delay 0.2)
        (Variables|Default|SetisInvicible false)))
    (Development|PrintString (Utilities|String|ToString(Integer) (Variables|Default|GetHP)))
    (CallFunction|FacePlayer)))

(event Custom|HitstunRecover
  (Variables|Default|SethitStun false))

(event Custom|SetNil
  (bind _asnil_bp (Utilities|Casting|CastToNil_BP (Game|Player|GetPlayerPawn 0))
    (:then
      (Variables|Default|SetNil _asnil_bp)
      (Development|PrintString "Succeeded to cast?"))
    (:CastFailed
      (Development|PrintString "Failed to Cast?"))))

(event Custom|FacePlayer
  (bind _returnvalue (Game|Player|GetPlayerPawn 0))
  (bind _returnvalue_2 (Transformation|GetActorLocation))
  (bind _returnvalue_3 (Transformation|GetActorLocation _returnvalue))
  (bind _returnvalue_4 (Math|Rotator|FindLookatRotation _returnvalue_2 _returnvalue_3))
  (bind (_roll _pitch _yaw) (Math|Rotator|BreakRotator _returnvalue_4))
  (Transformation|SetActorRotation (Math|Rotator|MakeRotator _roll (.Pitch (Math|Rotator|BreakRotator (Transformation|GetActorRotation))) _yaw)))

(event Custom|TakeKnockback
  (params (Knockback :type Integer) (Attacker :type Actor%20Object%20Reference))
  ;[1 1 1] Apply Knockback to Enemy
  (Character|LaunchCharacter (* (+ (- (Transformation|GetActorLocation) (Transformation|GetActorLocation Attacker)) "0, 0,65.000000") (Math|Conversions|ToFloat(Integer) (- Knockback (Variables|Default|GetKnockbackDef)))) true true)
  (AI|Navigation|StopMovement (AI|GetAIController self)))

(event EventBeginPlay)

(event Collision|EventActorBeginOverlap
  (params (OtherActor :type Actor%20Object%20Reference)))

(event EventTick
  (params (DeltaSeconds :type Float%20%28single-precision%29)))

(fn ConstructionScript)

(fn ToggleIgnorePlayer
  (params (On/Off :type Boolean))
  (bind _nil (Variables|Default|GetNil))
  (Collision|IgnoreActorwhenMoving (Variables|Collision|GetCapsuleComponent) _nil On/Off)
  (Collision|IgnoreActorwhenMoving (Variables|/Script/Engine.Character|GetCapsuleComponent _nil) self On/Off))