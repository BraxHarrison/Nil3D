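; Candle actor in the cave room that can be lit once by a MarshWad_BP actor.
; When a MarshWad_BP with ShouldKill set overlaps LightBox, LightCandle shows the Flame and unhides the PointLight, and IsLit blocks repeat triggers.
; Lighting then calls LightTorch on every HiddenBlock actor in the level, found with GetAllActorsOfClass.
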(event OnComponentBeginOverlap(LightBox)
  (params (OverlappedComponent :type Primitive%20Component%20Object%20Reference) (OtherActor :type Actor%20Object%20Reference) (OtherComp :type Primitive%20Component%20Object%20Reference) (OtherBodyIndex :type Integer) (bFromSweep :type Boolean) (SweepResult :type Hit%20Result%20Structure%20%28by%20ref%29))
  (if (not (Variables|Default|GetisLit))
    (bind _asmarsh_wad_bp (Utilities|Casting|CastToMarshWad_BP OtherActor))
    (if (Variables|/Game/Actors/Enemies/Projectiles_Master.Projectiles_Master_C|GetshouldKill _asmarsh_wad_bp)
      (CallFunction|LightCandle)
      (Variables|Default|SetisLit true)
      (bind _outactors (Actor|GetAllActorsOfClass "/Game/Levels/CaveRoom/Meshes/HiddenBlock.HiddenBlock_C"))
      (for _array_element _outactors
        (Default|LightTorch _array_element)))))

(event Custom|LightCandle
  (Rendering|SetVisibility (Variables|Default|GetFlame) true false)
  (Development|SetHiddeninGame (Variables|Default|GetPointLight) false false))

(event EventBeginPlay)

(event Collision|EventActorBeginOverlap
  (params (OtherActor :type Actor%20Object%20Reference)))

(event EventTick
  (params (DeltaSeconds :type Float%20%28single-precision%29)))

(fn ConstructionScript)