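; Scarf tree in the opening area: a talking scarf stuck on a branch that the player activates to collect, once per save.
; Timed speech bubble lines call for help and enable activation.
; Activating shows the scarf on the player, clears the tree's scarf material and moves dialogue to the player's billboard for backstory.
; Completion saves through the game instance, so later loads skip the conversation and hide the scarf.
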(event Custom|LoadLevelState
  (bind _asnil_gi (Utilities|Casting|CastToNil_GI (Game|GetGameInstance)))
  (Variables|Default|SeteventCompleted (Variables|/Game/System/SaveGame_BP.SaveGame_BP_C|GetscarfCollected (Variables|/Game/System/Nil_GI.Nil_GI_C|GetlastSave _asnil_gi))))

(event Custom|SaveLevelState
  (bind _asnil_gi (Utilities|Casting|CastToNil_GI (Game|GetGameInstance)))
  (Variables|/Game/System/SaveGame_BP.SaveGame_BP_C|SetscarfCollected (Variables|/Game/System/Nil_GI.Nil_GI_C|GetlastSave _asnil_gi) (Variables|Default|GeteventCompleted))
  (Default|TryMakeSave _asnil_gi))

(event Custom|CollectScarf
  (bind _asnil_bp (Utilities|Casting|CastToNil_BP (Game|Player|GetPlayerPawn 0)))
  (Default|ToggleScarf _asnil_bp true)
  (Rendering|Material|SetMaterial (Variables|Default|GetScarfTree) 1 "/Game/Levels/CaveRoom/Meshes/Candle/Nothing.Nothing"))

(event EventBeginPlay
  (CallFunction|LoadLevelState)
  (if (Variables|Default|GeteventCompleted)
    (Rendering|Material|SetMaterial (Variables|Default|GetScarfTree) 1 "/Game/Levels/CaveRoom/Meshes/Candle/Nothing.Nothing")
    (else
      (CallFunction|StartConversation))))

(event Collision|EventActorBeginOverlap
  (params (OtherActor :type Actor%20Object%20Reference)))

(event EventTick
  (params (DeltaSeconds :type Float%20%28single-precision%29)))

(event EventActivate
  (|CallParentFunction)
  (if (Variables|Default|GetcanActivate)
    (CallFunction|CollectScarf)
    (Default|EndConversation (Variables|Default|GetspeechBubble))
    (CallFunction|Speech2)))

(event Custom|StartConversation
  (bind _asnil_gi (Utilities|Casting|CastToNil_GI (Game|GetGameInstance)))
  (bind _output_get (Variables|Default|SetspeechBubble (Variables|/Game/System/Nil_GI.Nil_GI_C|GetSpeechBubble _asnil_gi)))
  (Default|StartConversation _output_get (Variables|Default|GetBillboard) 1.5e+02)
  (UserInterface|Viewport|AddtoViewport _output_get 0)
  (CallFunction|Speech))

(event Custom|Speech
  (bind _speechbubble (Variables|Default|GetspeechBubble))
  (Default|FeedText _speechbubble "Hey! Kid! A little help here?")
  (Utilities|FlowControl|Delay 3.0)
  (Default|FeedText _speechbubble "Come over here and use Q to get me down off of this branch!")
  (Variables|Default|SetcanActivate true))

(event Custom|Speech2
  (bind _speechbubble (Variables|Default|GetspeechBubble))
  (bind _asnil_bp (Utilities|Casting|CastToNil_BP (Game|Player|GetPlayerPawn 0)))
  (Default|StartConversation _speechbubble (Variables|/Game/Actors/Player/Nil_BP.Nil_BP_C|GetBillboard _asnil_bp) 25.0)
  (Default|FeedText _speechbubble "Thanks a bunch, kid. ")
  (Utilities|FlowControl|Delay 1.0)
  (Default|FeedText _speechbubble "So here's the deal: me and my owner got the stuffing beat out of us pretty bad.")
  (Utilities|FlowControl|Delay 3.0)
  (Default|FeedText _speechbubble "Our attackers had some kind of weird weapon. I think they sapped all of my spirit energy.")
  (Utilities|FlowControl|Delay 3.0)
  (Default|FeedText _speechbubble "But my owner busted it up and my spirits went all over the place. It looks like one landed on that ledge over there. ")
  (Variables|Default|SeteventCompleted true)
  (CallFunction|SaveLevelState)
  (Utilities|FlowControl|Delay 3.0)
  (Default|EndConversation (Variables|Default|GetspeechBubble)))

(fn ConstructionScript)